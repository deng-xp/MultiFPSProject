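; BP_SFPSCharacter is a player character Blueprint that sets up the local player's HUD and shows a health debug readout.
; On BeginPlay, if locally controlled, it creates the crosshair and health widgets and adds them to the viewport.
; On Tick, also only when locally controlled, it reads the HealthComponent's health and prints it on screen each frame without logging.
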(event EventTick
  (params (DeltaSeconds :type Float%20%28single-precision%29))
  (if (Pawn|IsLocallyControlled)
    (bind _returnvalue (Class|SHealthComponent|GetHealth (Variables|Default|GetHealthComponent)))
    (Development|PrintString (Utilities|String|ToString(Float) _returnvalue) true false "(R=0.436197,G=1.000000,B=0.172612,A=1.000000)" 0.0)))

(event EventBeginPlay
  (if (Pawn|IsLocallyControlled)
    (Utilities|FlowControl|Sequence
      (:then_0
        (bind _returnvalue (UserInterface|CreateWidget "/Game/UI/WBP_Crosshair.WBP_Crosshair_C"))
        (UserInterface|Viewport|AddtoViewport _returnvalue 0))
      (:then_1
        (bind _returnvalue_2 (UserInterface|CreateWidget "/Game/UI/WBP_Health.WBP_Health_C"))
        (UserInterface|Viewport|AddtoViewport _returnvalue_2 0)))))

(fn ConstructionScript)